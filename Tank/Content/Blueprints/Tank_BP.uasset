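; Player-controllable tank Blueprint that wires up its components and routes driving, camera aim and fire input.
; On BeginPlay it registers the Turret and Barrel references and initialises TankMovement with the left and right tracks.
; Drive axes feed movement intents to TankMovement, while Fire calls the tank's Fire function.
; Aim axes split rotation across two components: yaw on AzimuthGimbal and pitch on SpringArm, leaving turret and barrel untouched here.
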(event `self.ReceiveBeginPlay`
  (`self.SetTurretReference` (`self.Turret`))
  (`self.SetBarrelReference` (`self.Barrel`))
  (`TankMovementComponent.Initialise` (`self.TankMovement`) (`self.Left Track`) (`self.Right Track`)))

(event `InputAxis|AimAzimuth`
  (params (AxisValue :type "Float (single-precision)"))
  ;[1 1 1] Aim Input Binding
  (`SceneComponent.K2_AddLocalRotation` (`self.AzimuthGimbal`) (`KismetMathLibrary.MakeRotator` 0.0 0.0 AxisValue) false false))

(event `InputAxis|Forward and Back`
  (params (AxisValue :type "Float (single-precision)"))
  ;[1 1 1] Movement Input Binding
  (`TankMovementComponent.IntendMoveForward` (`self.TankMovement`) AxisValue))

(event `InputAxis|AimElevation`
  (params (AxisValue :type "Float (single-precision)"))
  ;[1 1 1] Aim Input Binding
  (`SceneComponent.K2_AddLocalRotation` (`self.SpringArm`) (`KismetMathLibrary.MakeRotator` 0.0 AxisValue) false false))

(event `InputAxis|Turn Right`
  (params (AxisValue :type "Float (single-precision)"))
  ;[1 1 1] Movement Input Binding
  (`TankMovementComponent.IntendTurnRight` (`self.TankMovement`) AxisValue))

(event `InputAction|Fire`
  (params (Key :type "Key Structure"))
  ;[1 1 1] Aim Input Binding
  (:`Pressed`
    (`self.Fire`)))

(fn `UserConstructionScript`)